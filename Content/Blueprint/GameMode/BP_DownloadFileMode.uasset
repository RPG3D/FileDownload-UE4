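; Game mode Blueprint that runs a file download screen with a start/stop control.
; On BeginPlay it shows a DownloadWidget with the mouse cursor and constructs a FileDownloadManager object.
; Manager events push the task's info into the widget, while the widget's start/stop event starts or stops all downloads.
; EndPlay clears the manager reference.
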(event `self.ReceiveBeginPlay`
  (bind _returnvalue (`GameplayStatics.GetPlayerController` 0))
  (`|ExecutionSequence`
    (:`then_0`
      ;[1 1 1] CreateUI
      (bind _returnvalue_2 (`|CreateWidget` "/Game/UI/Download/DownloadWidget.DownloadWidget_C" _returnvalue))
      (bind _output_get (set `self.dlWidget` _returnvalue_2))
      (`UserWidget.AddToViewport` _output_get 0)
      (set `PlayerController.bShowMouseCursor` true _returnvalue))
    (:`then_1`
      ;[1 1 1] CreateDownloadManager
      (bind _returnvalue_3 (`|GenericCreateObject` self "/Script/FileDownloader.FileDownloadManager"))
      (set `self.DlManager` _returnvalue_3))
    (:`then_2`
      ;[1 1 1] BindEvent
      (add `FileDownloadManager.OnDlManagerEvent` (`self.DlManager`) (delegate `CustomEvent_0`))
      (add `/Game/UI/Download/DownloadWidget.StartOrStop` (`self.dlWidget`) (delegate `CustomEvent_1`)))))

(event `CustomEvent_0`
  (params (InEvent :type "ETaskEvent Enum" :default "START_DOWNLOAD") (InTaskID :type Integer) (InHttpCode :type Integer))
  ;[1 1 1] BindEvent
  (`/Game/UI/Download/DownloadWidget.ProcessInfoChanged` (`self.dlWidget`) InEvent (`FileDownloadManager.GetTaskInfo` (`self.DlManager`) InTaskID)))

(event `CustomEvent_1`
  (params (bShouldStart :type Boolean))
  (bind _dlmanager (`self.DlManager`))
  ;[1 1 1] BindEvent
  (if bShouldStart
    (`FileDownloadManager.StartAll` _dlmanager)
    (else
      (`FileDownloadManager.StopAll` _dlmanager))))

(event `self.ReceiveEndPlay`
  (params (EndPlayReason :type "EEndPlayReason Enum" :default "Destroyed"))
  (set `self.DlManager` null))

(fn `UserConstructionScript`)